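; BP_BaseTetrisPawn is a base pawn for a Tetris game that handles camera look control.
; The LookHorizontally and LookVertically axis inputs add relative yaw and pitch to the spring arm.
; Pitch input is ignored when it would push the arm beyond 80 degrees up or down.
; BeginPlay, Tick, overlap and the construction script are empty, and a leftover rotator debug print is unconnected.
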(event `InputAxis|LookHorizontally`
  (params (AxisValue :type "Float (single-precision)"))
  (`SceneComponent.K2_AddRelativeRotation` (`self.SpringArmComponent`) (`KismetMathLibrary.MakeRotator` 0.0 0.0 AxisValue) false false))

(event `InputAxis|LookVertically`
  (params (AxisValue :type "Float (single-precision)"))
  (bind _springarmcomponent (`self.SpringArmComponent`))
  (bind (_relativerotation_roll _relativerotation_pitch) (`KismetMathLibrary.BreakRotator` (`SceneComponent.RelativeRotation` _springarmcomponent)))
  (if (not (> (`KismetMathLibrary.Abs` (+ _relativerotation_pitch AxisValue)) 80.0))
    (`SceneComponent.K2_AddRelativeRotation` _springarmcomponent (`KismetMathLibrary.MakeRotator` 0.0 AxisValue) false false)))

(event `self.ReceiveTick`
  (params (DeltaSeconds :type "Float (single-precision)")))

(fn `UserConstructionScript`)